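; BP_Button is an on/off pressure button that stays pressed while actors overlap its trigger and switches a linked object.
; Overlap begin plays the Push timeline to move the button along Z, and overlap end reverses it once no actors remain.
; When the timeline finishes in either direction, the button turns green or red and sends its Pressed state to ObjectToAffect via TurnSwitchMessage.
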(event OnComponentBeginOverlap(Trigger)
  (params (OverlappedComponent :type Primitive%20Component%20Object%20Reference) (OtherActor :type Actor%20Object%20Reference) (OtherComp :type Primitive%20Component%20Object%20Reference) (OtherBodyIndex :type Integer) (bFromSweep :type Boolean) (SweepResult :type Hit%20Result%20Structure%20%28by%20ref%29))
  (if (not (Variables|Default|GetPressed))
    (Variables|Default|SetPressed true)
    ;[1 1 1] Animation
    (bind _push (Timeline|Push Play)
      (:Update
        (Transformation|SetRelativeLocation (Variables|Default|GetButton) (Math|Vector|MakeVector 0.0 0.0 _push) false false))
      (:Finished
        (if (Variables|Default|GetPressed)
          ;[1 1 1] Material
          (Rendering|Material|SetMaterial (Variables|Default|GetButton) 0 "/Game/OwnMaterial/Green.Green")
          (else
            (Rendering|Material|SetMaterial (Variables|Default|GetButton) 0 "/Game/OwnMaterial/Red.Red")))
        (Class|BPTurnSwitch|TurnSwitch(Message) (Variables|Default|GetObjectToAffect) (Variables|Default|GetPressed))))))

(event OnComponentEndOverlap(Trigger)
  (params (OverlappedComponent :type Primitive%20Component%20Object%20Reference) (OtherActor :type Actor%20Object%20Reference) (OtherComp :type Primitive%20Component%20Object%20Reference) (OtherBodyIndex :type Integer))
  (if (not (Utilities|Array|IsValidIndex (Collision|GetOverlappingActors (Variables|Default|GetTrigger) 0 :!class /Script/Engine.PrimitiveComponent)))
    (Variables|Default|SetPressed false)
    ;[1 1 1] Animation
    (bind _push (Timeline|Push Reverse)
      (:Update
        (Transformation|SetRelativeLocation (Variables|Default|GetButton) (Math|Vector|MakeVector 0.0 0.0 _push) false false))
      (:Finished
        (if (Variables|Default|GetPressed)
          ;[1 1 1] Material
          (Rendering|Material|SetMaterial (Variables|Default|GetButton) 0 "/Game/OwnMaterial/Green.Green")
          (else
            (Rendering|Material|SetMaterial (Variables|Default|GetButton) 0 "/Game/OwnMaterial/Red.Red")))
        (Class|BPTurnSwitch|TurnSwitch(Message) (Variables|Default|GetObjectToAffect) (Variables|Default|GetPressed))))))

(fn ConstructionScript)