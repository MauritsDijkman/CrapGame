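; BP_Platform is a switch-driven platform actor that appears or disappears in response to a TurnSwitch event.
; The TurnOn flag sets its polarity: when true it starts hidden and shows while the switch is active, when false it does the reverse.
; BeginPlay applies the starting state, and each change toggles both actor visibility and the Cube's collision, so a hidden platform is not solid.
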(event EventTurnSwitch
  (params (Active? :type Boolean))
  ;[1 1 1] Enable/Disable
  (if Active?
    (if (Variables|Default|GetTurnOn)
      (Rendering|SetActorHiddenInGame false :!label _label)
      (Collision|SetCollisionEnabled (Variables|Default|GetCube) "QueryAndPhysics")
      (else
        (Rendering|SetActorHiddenInGame true :!label _label_2)
        (Collision|SetCollisionEnabled (Variables|Default|GetCube) "NoCollision")))
    (elif (Variables|Default|GetTurnOn)
      (goto _label_2)
      (else
        (goto _label)))))

(event EventBeginPlay
  ;[1 1 1] StartCode
  (if (Variables|Default|GetTurnOn)
    (Rendering|SetActorHiddenInGame true)
    (Collision|SetCollisionEnabled (Variables|Default|GetCube) "NoCollision")
    (else
      (Rendering|SetActorHiddenInGame false)
      (Collision|SetCollisionEnabled (Variables|Default|GetCube) "QueryAndPhysics"))))

(fn ConstructionScript
  ;[1 1 1] Standard
  (|CallParentFunction))