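; Moving platform actor that travels between two relative points and can appear or vanish in response to a switch.
; The construction script feeds Location1, Location2 and Duration into an InterpToMovement component.
; TurnOn makes the platform start hidden without collision and appear when TurnSwitch is active; otherwise it starts solid and vanishes when active.
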(event EventTurnSwitch
  (params (Active? :type Boolean))
  ;[1 1 1] Enable/Disable
  (if Active?
    (if (Variables|Default|GetTurn%20On)
      (Rendering|SetActorHiddenInGame false :!label _label)
      (Collision|SetCollisionEnabled (Variables|Default|GetPlatform) "QueryAndPhysics")
      (else
        (Rendering|SetActorHiddenInGame true :!label _label_2)
        (Collision|SetCollisionEnabled (Variables|Default|GetPlatform) "NoCollision")))
    (elif (Variables|Default|GetTurn%20On)
      (goto _label_2)
      (else
        (goto _label)))))

(event EventBeginPlay
  ;[1 1 1] StartCode
  (if (Variables|Default|GetTurn%20On)
    (Rendering|SetActorHiddenInGame true)
    (Collision|SetCollisionEnabled (Variables|Default|GetPlatform) "NoCollision")
    (else
      (Rendering|SetActorHiddenInGame false)
      (Collision|SetCollisionEnabled (Variables|Default|GetPlatform) "QueryAndPhysics"))))

(fn ConstructionScript
  (bind _interptomovement (Variables|Default|GetInterpToMovement))
  ;[1 1 1] Moving platform
  (Variables|/Script/Engine.InterpToMovementComponent|SetControlPoints _interptomovement (Utilities|Array|MakeArray (Utilities|Struct|MakeInterpControlPoint (Variables|Default|GetLocation_1) true) (Utilities|Struct|MakeInterpControlPoint (Variables|Default|GetLocation_2) true)))
  (Variables|/Script/Engine.InterpToMovementComponent|SetDuration _interptomovement (Variables|Default|GetDuration)))